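; BP_EnemyFlame is an enemy that chases the player when seen via PawnSensing and AIMoveTo.
; A looping timer fires a forward line trace that damages the player, resets their combo and shows the game-over widget at zero health.
; Overlapping the player while they attack or slide ragdolls the enemy with particles and a force along its arrow; only attacks build the player's combo meter.
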(event OnSeePawn(PawnSensing)
  (params (Pawn :type Pawn%20Object%20Reference))
  ;[1 1 1] Move towards player
  (bind _asbp_third_person_character (Utilities|Casting|CastToBP_ThirdPersonCharacter Pawn))
  (AI|AIMoveTo self "0, 0, 0" _asbp_third_person_character 5.0 false))

(event OnComponentBeginOverlap(CapsuleComponent)
  (params (OverlappedComponent :type Primitive%20Component%20Object%20Reference) (OtherActor :type Actor%20Object%20Reference) (OtherComp :type Primitive%20Component%20Object%20Reference) (OtherBodyIndex :type Integer) (bFromSweep :type Boolean) (SweepResult :type Hit%20Result%20Structure%20%28by%20ref%29))
  (bind _mesh (Variables|Character|GetMesh))
  (bind _capsulecomponent (Variables|Collision|GetCapsuleComponent))
  ;[1 1 1] Check if player overlaps
  (bind _output_get (Variables|Default|SetOverlap%20Actor%20 OtherActor))
  (if (== (Utilities|GetClass _output_get) (Variables|Default|GetPlayerClassRef))
    (Utilities|FlowControl|Sequence
      (:then_0
        ;[1 1 1] Check if attack button is pressed
        (bind _asbp_third_person_character (Utilities|Casting|CastToBP_ThirdPersonCharacter (Game|GetPlayerCharacter 0)))
        (if (Variables|/Game/Blueprints/BP_ThirdPersonCharacter.BP_ThirdPersonCharacter_C|GetIsAttackPressed _asbp_third_person_character)
          ;[1 1 1] Adding one to the combo, checking whether combo is full.
          (Audio|PlaySound2D "/Game/Audio/BITCHSLAP.BITCHSLAP" 1.0 1.0 0.0 0 0)
          (bind _output_get_2 (Variables|/Game/Blueprints/BP_ThirdPersonCharacter.BP_ThirdPersonCharacter_C|SetComboMeter _asbp_third_person_character (+ (Variables|/Game/Blueprints/BP_ThirdPersonCharacter.BP_ThirdPersonCharacter_C|GetComboMeter _asbp_third_person_character) 1.0)))
          (if (>= _output_get_2 (Variables|/Game/Blueprints/BP_ThirdPersonCharacter.BP_ThirdPersonCharacter_C|GetMaxCombo _asbp_third_person_character))
            (Variables|/Game/Blueprints/BP_ThirdPersonCharacter.BP_ThirdPersonCharacter_C|SetComboMeterFull _asbp_third_person_character true))
          ;[1 1 1] enable ragdoll
          (Physics|SetSimulatePhysics _capsulecomponent false :!label _label)
          (Collision|SetCollisionResponsetoChannel _capsulecomponent "ECC_PhysicsBody" "ECR_Ignore")
          (Class|SkeletalMeshComponent|SetAllBodiesBelowSimulatePhysics _mesh (Class|SkinnedMeshComponent|GetBoneName _mesh 1) true true)
          (Collision|SetCollisionEnabled (Variables|Collision|GetCapsuleComponent) "NoCollision")
          ;[1 1 1] Particles
          (Components|Activation|Activate (Variables|Default|GetParticleSystem) false)
          ;[1 1 1] Add force
          (Physics|AddForce (Variables|Character|GetMesh) (* (Math|Vector|GetForwardVector (Variables|Default|GetArrow1)) (Variables|Default|GetForceAddedF)) "None" false)))
      (:then_1
        ;[1 1 1] Check if player is in slide mode, then attack
        (bind _asbp_third_person_character_2 (Utilities|Casting|CastToBP_ThirdPersonCharacter (Game|GetPlayerCharacter 0)))
        (if (Variables|/Game/Blueprints/BP_ThirdPersonCharacter.BP_ThirdPersonCharacter_C|GetIsSlideActivated _asbp_third_person_character_2)
          (goto _label))))))

(event Custom|Attack
  (bind _arrow1 (Variables|Default|GetArrow1))
  (bind _returnvalue (Transformation|GetWorldLocation _arrow1))
  ;[1 1 1] Attack Logic
  (bind _outhit (Collision|LineTraceByChannel _returnvalue (+ _returnvalue (* (Math|Vector|GetForwardVector _arrow1) (Variables|Default|GetRange))) "TraceTypeQuery1" false 0 "ForDuration"))
  (bind _output_get (Variables|Default|SetOverlap%20Actor%20Attack (.hitactor _outhit)))
  (if (== (Utilities|GetClass _output_get) (Variables|Default|GetPlayerClassRef))
    (bind _asbp_third_person_character (Utilities|Casting|CastToBP_ThirdPersonCharacter (Game|GetPlayerCharacter 0)))
    (Variables|/Game/Blueprints/BP_ThirdPersonCharacter.BP_ThirdPersonCharacter_C|SetComboMeter _asbp_third_person_character 0.0)
    (Variables|/Game/Blueprints/BP_ThirdPersonCharacter.BP_ThirdPersonCharacter_C|SetComboMeterFull _asbp_third_person_character false)
    (bind _output_get_2 (Variables|/Game/Blueprints/BP_ThirdPersonCharacter.BP_ThirdPersonCharacter_C|SetHealth _asbp_third_person_character (- (Variables|/Game/Blueprints/BP_ThirdPersonCharacter.BP_ThirdPersonCharacter_C|GetHealth _asbp_third_person_character) (Variables|Default|GetDamage))))
    (Development|PrintString (Utilities|String|ToString(Float) _output_get_2))
    (Audio|PlaySound2D "/Game/Audio/Smoll_Boi_Ouch.Smoll_Boi_Ouch" 1.0 1.0 0.0 0 0)
    (if (<= _output_get_2 0.0)
      (bind _returnvalue_2 (UserInterface|CreateWidget "/Game/Widgets/W_GameOver.W_GameOver_C"))
      (UserInterface|Viewport|AddtoViewport _returnvalue_2 0))))

(event EventBeginPlay
  ;[1 1 1] Activate attack on timer
  (CallFunction|Attack :!label _label)
  (Utilities|FlowControl|Delay (Variables|Default|GetAttack%20Timer))
  (goto _label))

(fn ConstructionScript)