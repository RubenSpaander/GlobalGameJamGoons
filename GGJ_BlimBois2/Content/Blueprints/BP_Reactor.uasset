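; BP_Reactor is a damageable reactor that serves as the game's win condition.
; When an actor of the PlayerRef class enters its sphere, it plays a 2D sound and checks IsActive on the player's BP_ThirdPersonCharacter.
; If active, each overlap subtracts ReactorDamage from ReactorHealth, and the W_Win widget is shown once health is zero or below.
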(event OnComponentBeginOverlap(Sphere)
  (params (OverlappedComponent :type Primitive%20Component%20Object%20Reference) (OtherActor :type Actor%20Object%20Reference) (OtherComp :type Primitive%20Component%20Object%20Reference) (OtherBodyIndex :type Integer) (bFromSweep :type Boolean) (SweepResult :type Hit%20Result%20Structure%20%28by%20ref%29))
  ;[1 1 1] Win condition
  (bind _output_get (Variables|Default|SetActorRefReactor OtherActor))
  (if (== (Utilities|GetClass _output_get) (Variables|Default|GetPlayerRef))
    (Audio|PlaySound2D "/Game/Audio/Audio_files/KANKERGROTEBOEM.KANKERGROTEBOEM" 1.0 1.0 0.0 0 0)
    (bind _asbp_third_person_character (Utilities|Casting|CastToBP_ThirdPersonCharacter (Game|GetPlayerCharacter 0)))
    (if (Variables|/Game/Blueprints/BP_ThirdPersonCharacter.BP_ThirdPersonCharacter_C|GetIsActive _asbp_third_person_character)
      (bind _output_get_2 (Variables|Default|SetReactorHealth (- (Variables|Default|GetReactorHealth) (Variables|Default|GetReactor%20Damage))))
      (if (<= _output_get_2 0.0)
        (bind _returnvalue (UserInterface|CreateWidget "/Game/Widgets/W_Win.W_Win_C"))
        (UserInterface|Viewport|AddtoViewport _returnvalue 0)))))

(fn ConstructionScript)