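; BP_Spawner is an actor that keeps the level populated with BP_Enemy AI pawns inside a spawn box.
; On BeginPlay it starts a looping timer at SpawnTime intervals.
; Each tick of the timer counts all BP_Enemy actors in the level and, while below AmountOfEnemy, spawns one at a random point within the SpawnBox bounds.
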(event Custom|SpawnAI
  (bind _spawnbox (Variables|Default|GetSpawnBox))
  (bind _outactors (Actor|GetAllActorsOfClass "/Game/Blueprints/BP_Enemy.BP_Enemy_C"))
  (if (<= (Utilities|Array|Length _outactors) (- (Variables|Default|GetAmount%20of%20Enemy) 1))
    (AI|SpawnAIFromClass "/Game/Blueprints/BP_Enemy.BP_Enemy_C" 0 (Math|Random|RandomPointinBoundingBox (Transformation|GetWorldLocation _spawnbox) (Components|Box|GetScaledBoxExtent _spawnbox)) "0, 0, 0" false)))

(event EventBeginPlay
  (Utilities|Time|SetTimerbyEvent (delegate Custom|SpawnAI) (Variables|Default|GetSpawnTime) true))

(fn ConstructionScript)