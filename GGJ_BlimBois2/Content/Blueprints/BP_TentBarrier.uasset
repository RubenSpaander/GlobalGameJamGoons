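; BP_TentBarrier is a barrier actor that is destroyed when the player slides into it.
; On box overlap, it compares the overlapping actor's class to a stored class, then reads the slide state from player 0's BP_ThirdPersonCharacter.
; If the slide is active, it zeroes the character's TimeOfBoost and destroys itself; otherwise the overlap has no further effect.
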(event OnComponentBeginOverlap(Box)
  (params (OverlappedComponent :type Primitive%20Component%20Object%20Reference) (OtherActor :type Actor%20Object%20Reference) (OtherComp :type Primitive%20Component%20Object%20Reference) (OtherBodyIndex :type Integer) (bFromSweep :type Boolean) (SweepResult :type Hit%20Result%20Structure%20%28by%20ref%29))
  (bind _output_get (Variables|Default|SetPlayer%20Ref%20Tent OtherActor))
  (if (== (Utilities|GetClass _output_get) (Variables|Default|GetPlayer%20Ref%20Tent%20Class))
    (bind _asbp_third_person_character (Utilities|Casting|CastToBP_ThirdPersonCharacter (Game|GetPlayerCharacter 0)))
    (if (Variables|/Game/Blueprints/BP_ThirdPersonCharacter.BP_ThirdPersonCharacter_C|GetIsSlideActivated _asbp_third_person_character)
      (Variables|/Game/Blueprints/BP_ThirdPersonCharacter.BP_ThirdPersonCharacter_C|SetTimeOfBoost _asbp_third_person_character 0.0)
      (Actor|DestroyActor))))

(fn ConstructionScript)