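; ZoneStart is a zone trigger actor that switches on its assigned spawners when the player character leaves its overlap.
; It finds the level's ZoneManager on BeginPlay.
; On end overlap with BP_ThirdPersonCharacter, it flags every entry in Spawners as activated and passes itself to the manager's EnableZone.
; A separate DisableSpawners function calls StopSpawner on each of those spawners.
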(event EventBeginPlay
  (bind _outactors (Actor|GetAllActorsOfClass "/Game/Blueprints/ZoneManager.ZoneManager_C"))
  (Variables|Default|SetZoneManager (Utilities|Array|Get(acopy) _outactors)))

(event EventTick
  (params (DeltaSeconds :type Float%20%28single-precision%29)))

(event Collision|EventActorEndOverlap
  (params (OtherActor :type Actor%20Object%20Reference))
  (Utilities|Casting|CastToBP_ThirdPersonCharacter OtherActor)
  (for _array_element (Variables|Default|GetSpawners)
    (Variables|/Game/Blueprints/BP_Spawner.BP_Spawner_C|SetIsActivated _array_element true))
  (Default|EnableZone (Variables|Default|GetZoneManager) self))

(fn ConstructionScript)

(fn DisableSpawners
  (for _array_element (Variables|Default|GetSpawners)
    (Default|StopSpawner _array_element)))